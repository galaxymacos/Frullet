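; BP_Spawn is a spawn point actor that creates SimpleAI enemies at its own location.
; Its SpawnEnemy1 and SpawnEnemy2 functions are identical: each spawns the AI, then increments the EnemiesInScene counter on ThirdPersonGameMode.
; The event graph and construction script are empty, so nothing in this Blueprint triggers spawning itself.
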(fn `SpawnEnemy1`
  (`AIBlueprintHelperLibrary.SpawnAIFromClass` "/Game/ThirdPersonBP/Blueprints/Character/Ai/SimpleAI.SimpleAI_C" null (`self.K2_GetActorLocation`))
  (bind _asthird_person_game_mode (cast `/Game/ThirdPersonBP/Blueprints/ThirdPersonGameMode` (`GameplayStatics.GetGameMode`)))
  (`/Engine/EditorBlueprintResources/StandardMacros.IncrementInt` (`/Game/ThirdPersonBP/Blueprints/ThirdPersonGameMode.EnemiesInScene` _asthird_person_game_mode)))

(fn `SpawnEnemy2`
  (`AIBlueprintHelperLibrary.SpawnAIFromClass` "/Game/ThirdPersonBP/Blueprints/Character/Ai/SimpleAI.SimpleAI_C" null (`self.K2_GetActorLocation`))
  (bind _asthird_person_game_mode (cast `/Game/ThirdPersonBP/Blueprints/ThirdPersonGameMode` (`GameplayStatics.GetGameMode`)))
  (`/Engine/EditorBlueprintResources/StandardMacros.IncrementInt` (`/Game/ThirdPersonBP/Blueprints/ThirdPersonGameMode.EnemiesInScene` _asthird_person_game_mode)))

(fn `UserConstructionScript`)